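; BP_PlayerHoverCraft is the player-controlled hovercraft, handling basic throttle and steering through Enhanced Input.
; On BeginPlay it adds the controller input mapping context to its player controller's Enhanced Input subsystem.
; Acceleration applies movement input along the actor's forward vector at a fixed scale.
; Steering yaws the capsule component by the input value times RotationSpeed on each trigger, without delta-time scaling.
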(event Input|EnhancedActionEvents|EnhancedInputActionIA_Acceleration
  (params (ActionValue :type Float%20%28double-precision%29) (ElapsedSeconds :type Float%20%28double-precision%29) (TriggeredSeconds :type Float%20%28double-precision%29) (InputAction :type Input%20Action%20Object%20Reference :default "/Game/Niels/Input/IA_Acceleration.IA_Acceleration"))
  (:Triggered
    (Pawn|Input|AddMovementInput (Math|Vector|GetForwardVector (Transformation|GetActorRotation)) 1.0 false)))

(event Input|EnhancedActionEvents|EnhancedInputActionIA_SteerHovercraft
  (params (ActionValue :type Float%20%28double-precision%29) (ElapsedSeconds :type Float%20%28double-precision%29) (TriggeredSeconds :type Float%20%28double-precision%29) (InputAction :type Input%20Action%20Object%20Reference :default "/Game/Niels/Input/IA_SteerHovercraft.IA_SteerHovercraft"))
  (:Triggered
    (Transformation|AddRelativeRotation (Variables|Collision|GetCapsuleComponent) (Math|Rotator|MakeRotator 0.0 0.0 (* ActionValue (Variables|Default|GetrotationSpeed))) false false)))

(event EventBeginPlay
  (bind _asplayer_controller (Utilities|Casting|CastToPlayerController (Pawn|GetController)))
  (Utilities|IsValid (PlayerController|LocalPlayerSubsystems|GetEnhancedInputLocalPlayerSubsystem _asplayer_controller)
    (:Is%20Valid
      (Input|AddMappingContext (PlayerController|LocalPlayerSubsystems|GetEnhancedInputLocalPlayerSubsystem _asplayer_controller) "/Game/Niels/Input/IMC_ControllerInput.IMC_ControllerInput" 0 "(bIgnoreAllPressedKeysUntilRelease=True,bForceImmediately=False)"))))

(event Collision|EventActorBeginOverlap
  (params (OtherActor :type Actor%20Object%20Reference)))

(event EventTick
  (params (DeltaSeconds :type Float%20%28single-precision%29)))

(fn ConstructionScript)