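; Player pawn for a drivable hovercraft, moved by a FloatingPawnMovement component through Enhanced Input.
; Acceleration pushes along the yaw-and-roll right vector, steering yaws the static mesh, and drifting temporarily raises turning boost and rotation speed.
; Tick corrects roll and pitch to set limits and keeps the spring arm behind at a 90-degree yaw offset, except while camera-rotate input is held.
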(event Input|EnhancedActionEvents|EnhancedInputActionIA_Drifting
  (params (ActionValue :type Float%20%28double-precision%29) (ElapsedSeconds :type Float%20%28double-precision%29) (TriggeredSeconds :type Float%20%28double-precision%29) (InputAction :type Input%20Action%20Object%20Reference :default "/Game/Niels/Input/IA_Drifting.IA_Drifting"))
  ;[1 1 1] Drifting
  (:Triggered
    (Variables|/Script/Engine.FloatingPawnMovement|SetTurningBoost (Variables|Default|GetFloatingPawnMovement) 5.0)
    (Variables|Default|SetRotationSpeed 1.5))
  (:Completed
    (Variables|/Script/Engine.FloatingPawnMovement|SetTurningBoost (Variables|Default|GetFloatingPawnMovement) 0.5)
    (Variables|Default|SetRotationSpeed 1.0)))

(event Input|EnhancedActionEvents|EnhancedInputActionIA_Acceleration
  (params (ActionValue :type Float%20%28double-precision%29) (ElapsedSeconds :type Float%20%28double-precision%29) (TriggeredSeconds :type Float%20%28double-precision%29) (InputAction :type Input%20Action%20Object%20Reference :default "/Game/Niels/Input/IA_Acceleration.IA_Acceleration"))
  (bind _returnvalue (Transformation|GetActorRotation))
  (bind (_roll _pitch _yaw) (Math|Rotator|BreakRotator _returnvalue))
  ;[1 1 1] Accelerating
  (:Triggered
    (Class|PawnMovementComponent|AddInputVector (Variables|Default|GetFloatingPawnMovement) (* (Math|Vector|GetRightVector (Math|Rotator|MakeRotator _roll 0.0 _yaw)) (Variables|Default|GetSpeed)) false)))

(event Input|EnhancedActionEvents|EnhancedInputActionIA_RotateCamera
  (params (ActionValue :type Float%20%28double-precision%29) (ElapsedSeconds :type Float%20%28double-precision%29) (TriggeredSeconds :type Float%20%28double-precision%29) (InputAction :type Input%20Action%20Object%20Reference :default "/Game/Niels/Input/IA_RotateCamera.IA_RotateCamera"))
  (:Started
    (Variables|Default|SetControllingCamera true)
    (Transformation|SetWorldRotation (Variables|Default|GetSpringArm) (Math|Rotator|MakeRotator 0.0 0.0 (+ ActionValue (.Yaw (Math|Rotator|BreakRotator (Transformation|GetWorldRotation (Variables|Default|GetSpringArm)))))) false false))
  (:Completed
    (Development|PrintText "Input ended")
    (Variables|Default|SetControllingCamera false)))

(event Input|EnhancedActionEvents|EnhancedInputActionIA_SteerHovercraft
  (params (ActionValue :type Float%20%28double-precision%29) (ElapsedSeconds :type Float%20%28double-precision%29) (TriggeredSeconds :type Float%20%28double-precision%29) (InputAction :type Input%20Action%20Object%20Reference :default "/Game/Niels/Input/IA_SteerHovercraft.IA_SteerHovercraft"))
  ;[1 1 1] Steering
  (:Triggered
    (Transformation|AddRelativeRotation (Variables|Default|GetStaticMesh) (Math|Rotator|MakeRotator 0.0 0.0 (* ActionValue (Variables|Default|GetRotationSpeed))) false false)))

(event EventBeginPlay
  ;[1 1 1] Setup Input mapping
  (Utilities|FlowControl|Sequence
    (:then_0
      (bind _asplayer_controller (Utilities|Casting|CastToPlayerController (Pawn|GetController)))
      (Utilities|IsValid (PlayerController|LocalPlayerSubsystems|GetEnhancedInputLocalPlayerSubsystem _asplayer_controller)
        (:Is%20Valid
          (Input|AddMappingContext (PlayerController|LocalPlayerSubsystems|GetEnhancedInputLocalPlayerSubsystem _asplayer_controller) "/Game/Niels/Input/IMC_ControllerInput.IMC_ControllerInput" 0 "(bIgnoreAllPressedKeysUntilRelease=True,bForceImmediately=False)"))))
    (:then_1
      (Variables|/Script/Engine.FloatingPawnMovement|SetMaxSpeed (Variables|Default|GetFloatingPawnMovement) (Variables|Default|GetMaxSpeed)))))

(event Collision|EventActorBeginOverlap
  (params (OtherActor :type Actor%20Object%20Reference)))

(event EventTick
  (params (DeltaSeconds :type Float%20%28single-precision%29))
  (bind _returnvalue (Transformation|GetActorRotation))
  (bind _returnvalue_2 (Transformation|GetActorRotation))
  (bind _xrotmax (Variables|Default|GetxRotMax))
  (bind _yrotmax (Variables|Default|GetyRotMax))
  (bind (_roll _pitch _yaw) (Math|Rotator|BreakRotator _returnvalue))
  (bind (_roll_2 _pitch_2) (Math|Rotator|BreakRotator _returnvalue_2))
  ;[1 1 1] Clamp rotation
  (Transformation|AddRelativeRotation (Variables|Default|GetStaticMesh) (Math|Rotator|MakeRotator (- (Math|Float|ClampAngle _roll_2 (* _xrotmax -1.0) _xrotmax) _roll_2) (- (Math|Float|ClampAngle _pitch_2 (* _yrotmax -1.0) _yrotmax) _pitch_2) 0.0) false false)
  (if (not (Variables|Default|GetControllingCamera))
    (Transformation|SetWorldRotation (Variables|Default|GetSpringArm) (Math|Rotator|MakeRotator _roll _pitch (+ _yaw 9e+01)) false false)))

(fn ConstructionScript)