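; Player pawn for a drivable hovercraft, using Enhanced Input and FloatingPawnMovement with gravity added to velocity each tick.
; Input drives yaw-only forward thrust, low-speed reverse, mesh-rotation steering, and drifting that swaps turning boost and steering rate above a speed threshold.
; Tick scales camera FOV and shake with horizontal speed, easing FOV decreases.
; The spring arm lerps back to actor rotation unless under manual control, released after a short delay.
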(event Input|EnhancedActionEvents|EnhancedInputActionIA_Drifting
  (params (ActionValue :type Float%20%28double-precision%29) (ElapsedSeconds :type Float%20%28double-precision%29) (TriggeredSeconds :type Float%20%28double-precision%29) (InputAction :type Input%20Action%20Object%20Reference :default "/Game/Niels/Input/IA_Drifting.IA_Drifting"))
  (bind _returnvalue (Transformation|GetVelocity))
  (bind (_x _y) (Math|Vector|BreakVector _returnvalue))
  ;[1 1 1] Drifting
  (:Triggered
    (if (>= (Math|Vector|VectorLength (Math|Vector|MakeVector _x _y 0.0)) 1.5e+02)
      (Variables|/Script/Engine.FloatingPawnMovement|SetTurningBoost (Variables|Default|GetFloatingPawnMovement) (Variables|Default|GetDriftTurningBoost))
      (Variables|Default|SetSteeringMultiplier (Variables|Default|GetDriftRotSpeed))))
  (:Completed
    (Variables|/Script/Engine.FloatingPawnMovement|SetTurningBoost (Variables|Default|GetFloatingPawnMovement) (Variables|Default|GetTurningBoost))
    (Variables|Default|SetSteeringMultiplier (Variables|Default|GetRotationSpeed))))

(event Input|EnhancedActionEvents|EnhancedInputActionReverse
  (params (ActionValue :type Boolean) (ElapsedSeconds :type Float%20%28double-precision%29) (TriggeredSeconds :type Float%20%28double-precision%29) (InputAction :type Input%20Action%20Object%20Reference :default "/Game/Niels/Input/Reverse.Reverse"))
  (bind _returnvalue (Transformation|GetActorRotation))
  (bind _returnvalue_2 (Transformation|GetVelocity))
  (bind (_roll _pitch _yaw) (Math|Rotator|BreakRotator _returnvalue))
  (bind (_x _y) (Math|Vector|BreakVector _returnvalue_2))
  ;[1 1 1] Accelerating
  (:Triggered
    (if (>= 1.5e+02 (Math|Vector|VectorLength (Math|Vector|MakeVector _x _y 0.0)))
      (Class|PawnMovementComponent|AddInputVector (Variables|Default|GetFloatingPawnMovement) (* (Math|Vector|GetForwardVector (Math|Rotator|MakeRotator _roll 0.0 _yaw)) (* (Variables|Default|GetAcceleration) -1.0)) false))))

(event Input|EnhancedActionEvents|EnhancedInputActionIA_RotateCamera
  (params (ActionValue :type Float%20%28double-precision%29) (ElapsedSeconds :type Float%20%28double-precision%29) (TriggeredSeconds :type Float%20%28double-precision%29) (InputAction :type Input%20Action%20Object%20Reference :default "/Game/Niels/Input/IA_RotateCamera.IA_RotateCamera"))
  ;[1 1 1] Rotate Camera
  (:Triggered
    (Variables|Default|SetControllingCamera true)
    (Transformation|SetWorldRotation (Variables|Default|GetSpringArm) (Math|Rotator|MakeRotator 0.0 0.0 (+ ActionValue (.Yaw (Math|Rotator|BreakRotator (Transformation|GetWorldRotation (Variables|Default|GetSpringArm)))))) false false))
  (:Completed
    (Utilities|FlowControl|Delay 1.0)
    (Variables|Default|SetControllingCamera false)))

(event Input|EnhancedActionEvents|EnhancedInputActionIA_SteerHovercraft
  (params (ActionValue :type Float%20%28double-precision%29) (ElapsedSeconds :type Float%20%28double-precision%29) (TriggeredSeconds :type Float%20%28double-precision%29) (InputAction :type Input%20Action%20Object%20Reference :default "/Game/Niels/Input/IA_SteerHovercraft.IA_SteerHovercraft"))
  ;[1 1 1] Steering
  (:Triggered
    (Transformation|AddRelativeRotation (Variables|Default|GetStaticMesh) (Math|Rotator|MakeRotator 0.0 0.0 (* ActionValue (Variables|Default|GetSteeringMultiplier))) false false)))

(event Input|EnhancedActionEvents|EnhancedInputActionIA_Acceleration
  (params (ActionValue :type Float%20%28double-precision%29) (ElapsedSeconds :type Float%20%28double-precision%29) (TriggeredSeconds :type Float%20%28double-precision%29) (InputAction :type Input%20Action%20Object%20Reference :default "/Game/Niels/Input/IA_Acceleration.IA_Acceleration"))
  (bind _returnvalue (Transformation|GetActorRotation))
  (bind (_roll _pitch _yaw) (Math|Rotator|BreakRotator _returnvalue))
  ;[1 1 1] Accelerating
  (:Triggered
    (Class|PawnMovementComponent|AddInputVector (Variables|Default|GetFloatingPawnMovement) (* (Math|Vector|GetForwardVector (Math|Rotator|MakeRotator _roll 0.0 _yaw)) ActionValue (Variables|Default|GetAcceleration)) false)))

(event EventBeginPlay
  ;[1 1 1] Setup Input mapping
  (Utilities|FlowControl|Sequence
    (:then_0
      (bind _asplayer_controller (Utilities|Casting|CastToPlayerController (Pawn|GetController)))
      (Utilities|IsValid (PlayerController|LocalPlayerSubsystems|GetEnhancedInputLocalPlayerSubsystem _asplayer_controller)
        (:Is%20Valid
          (Input|AddMappingContext (PlayerController|LocalPlayerSubsystems|GetEnhancedInputLocalPlayerSubsystem _asplayer_controller) "/Game/Niels/Input/IMC_ControllerInput.IMC_ControllerInput" 0 "(bIgnoreAllPressedKeysUntilRelease=True,bForceImmediately=False)")
          (Variables|Default|SetSteeringMultiplier (Variables|Default|GetRotationSpeed)))))))

(event Collision|EventActorBeginOverlap
  (params (OtherActor :type Actor%20Object%20Reference)))

(event EventTick
  (params (DeltaSeconds :type Float%20%28single-precision%29))
  (bind _floatingpawnmovement (Variables|Default|GetFloatingPawnMovement))
  ;[1 1 1] Clamp rotation
  (Variables|/Script/Engine.MovementComponent|SetVelocity _floatingpawnmovement (+ (Variables|/Script/Engine.MovementComponent|GetVelocity _floatingpawnmovement) (* DeltaSeconds (Variables|Default|GetGravity))))
  (CallFunction|ApplyVisualEffects)
  (if (not (Variables|Default|GetControllingCamera))
    (CallFunction|ResetCameraPos)))

(fn ConstructionScript)

(fn ApplyVisualEffects
  (bind _maxspeed (Variables|Default|GetMaxSpeed))
  (bind _camera (Variables|Default|GetCamera))
  (bind _floatingpawnmovement (Variables|Default|GetFloatingPawnMovement))
  (bind _deltafov (Variables|Default|GetDeltaFOV))
  (bind _velocity (Variables|/Script/Engine.MovementComponent|GetVelocity _floatingpawnmovement))
  (bind _fieldofview (Variables|/Script/Engine.CameraComponent|GetFieldOfView _camera))
  (bind (_x _y) (Math|Vector|BreakVector _velocity))
  (bind _returnvalue (Math|Vector|MakeVector _x _y 0.0))
  (bind _returnvalue_2 (Math|Vector|VectorLength _returnvalue))
  (bind _returnvalue_3 (/ _returnvalue_2 _maxspeed))
  (bind _returnvalue_4 (* _returnvalue_3 _deltafov))
  (bind _returnvalue_5 (+ _returnvalue_4 9e+01))
  (if (>= (- _fieldofview _returnvalue_5) 1.0)
    (Camera|SetFieldOfView (Variables|Default|GetCamera) (Math|Float|Lerp _fieldofview _returnvalue_5 0.2))
    (else
      (Camera|SetFieldOfView (Variables|Default|GetCamera) _returnvalue_5)))
  (CameraShakes|StartCameraShake (Variables|Default|GetCameraShakeSource) "/Game/Niels/Blueprints/MyShakeBase.MyShakeBase_C" _returnvalue_4 "CameraLocal" "0, 0, 0"))

(fn ResetCameraPos
  (bind _returnvalue (Transformation|GetActorRotation))
  (bind (_roll _pitch _yaw) (Math|Rotator|BreakRotator _returnvalue))
  (Transformation|SetWorldRotation (Variables|Default|GetSpringArm) (Math|Rotator|Lerp(Rotator) (Transformation|GetWorldRotation (Variables|Default|GetSpringArm)) (Math|Rotator|MakeRotator _roll _pitch _yaw) 0.1 true) false false))