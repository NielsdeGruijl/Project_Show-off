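; Player-controlled hovercraft Character, driven through Enhanced Input with the controller mapping context and max walk speed set on BeginPlay.
; Acceleration adds movement along the actor's yaw-and-roll forward vector, while steering yaws the capsule by input times RotationSpeed, which drifting raises while held.
; Tick locks the spring arm to actor rotation with a 90-degree yaw offset; mesh pitch/roll clamping exists but is unconnected.
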(event Input|EnhancedActionEvents|EnhancedInputActionIA_Drifting
  (params (ActionValue :type Float%20%28double-precision%29) (ElapsedSeconds :type Float%20%28double-precision%29) (TriggeredSeconds :type Float%20%28double-precision%29) (InputAction :type Input%20Action%20Object%20Reference :default "/Game/Niels/Input/IA_Drifting.IA_Drifting"))
  ;[1 1 1] Drifting
  (:Triggered
    (Variables|Default|SetRotationSpeed 1.5))
  (:Completed
    (Variables|Default|SetRotationSpeed 1.0)))

(event Input|EnhancedActionEvents|EnhancedInputActionIA_Acceleration
  (params (ActionValue :type Float%20%28double-precision%29) (ElapsedSeconds :type Float%20%28double-precision%29) (TriggeredSeconds :type Float%20%28double-precision%29) (InputAction :type Input%20Action%20Object%20Reference :default "/Game/Niels/Input/IA_Acceleration.IA_Acceleration"))
  (bind _returnvalue (Transformation|GetActorRotation))
  (bind (_roll _pitch _yaw) (Math|Rotator|BreakRotator _returnvalue))
  ;[1 1 1] Accelerating
  (:Triggered
    (Pawn|Input|AddMovementInput (Math|Vector|GetForwardVector (Math|Rotator|MakeRotator _roll 0.0 _yaw)) 1.0 false)))

(event Input|EnhancedActionEvents|EnhancedInputActionIA_SteerHovercraft
  (params (ActionValue :type Float%20%28double-precision%29) (ElapsedSeconds :type Float%20%28double-precision%29) (TriggeredSeconds :type Float%20%28double-precision%29) (InputAction :type Input%20Action%20Object%20Reference :default "/Game/Niels/Input/IA_SteerHovercraft.IA_SteerHovercraft"))
  ;[1 1 1] Steering
  (:Triggered
    (Transformation|AddRelativeRotation (Variables|Collision|GetCapsuleComponent) (Math|Rotator|MakeRotator 0.0 0.0 (* ActionValue (Variables|Default|GetRotationSpeed))) false false)))

(event EventBeginPlay
  ;[1 1 1] Setup Input mapping
  (Utilities|FlowControl|Sequence
    (:then_0
      (bind _asplayer_controller (Utilities|Casting|CastToPlayerController (Pawn|GetController)))
      (Utilities|IsValid (PlayerController|LocalPlayerSubsystems|GetEnhancedInputLocalPlayerSubsystem _asplayer_controller)
        (:Is%20Valid
          (Input|AddMappingContext (PlayerController|LocalPlayerSubsystems|GetEnhancedInputLocalPlayerSubsystem _asplayer_controller) "/Game/Niels/Input/IMC_ControllerInput.IMC_ControllerInput" 0 "(bIgnoreAllPressedKeysUntilRelease=True,bForceImmediately=False)"))))
    (:then_1
      (Variables|/Script/Engine.CharacterMovementComponent|SetMaxWalkSpeed (Variables|Character|GetCharacterMovement) (Variables|Default|GetMaxSpeed)))))

(event Collision|EventActorBeginOverlap
  (params (OtherActor :type Actor%20Object%20Reference)))

(event EventTick
  (params (DeltaSeconds :type Float%20%28single-precision%29))
  (bind _returnvalue (Transformation|GetActorRotation))
  (bind (_roll _pitch _yaw) (Math|Rotator|BreakRotator _returnvalue))
  ;[1 1 1] Clamp rotation
  (Utilities|FlowControl|Sequence
    (:then_1
      (Transformation|SetWorldRotation (Variables|Default|GetSpringArm) (Math|Rotator|MakeRotator _roll _pitch (+ _yaw 9e+01)) false false))))

(fn ConstructionScript)