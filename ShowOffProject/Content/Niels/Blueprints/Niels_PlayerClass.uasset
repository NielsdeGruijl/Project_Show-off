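; Player pawn class for a hovercraft, driven through Enhanced Input with the controller mapping context added on BeginPlay.
; Look input feeds controller yaw and pitch, while acceleration adds full forward movement input along the actor's heading, ignoring pitch.
; Steering sets actor yaw directly by input times RotationSpeed, without delta-time scaling, zeroing pitch and roll.
; Yaw snaps to zero when the new value reaches 359 degrees or more.
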(event Input|EnhancedActionEvents|EnhancedInputActionIA_LookCharacter
  (params (ActionValue :type Vector%202D%20Structure) (ElapsedSeconds :type Float%20%28double-precision%29) (TriggeredSeconds :type Float%20%28double-precision%29) (InputAction :type Input%20Action%20Object%20Reference :default "/Game/Liam/Character/Input/IA_LookCharacter.IA_LookCharacter"))
  (:Triggered
    (Pawn|Input|AddControllerYawInput (.x ActionValue))
    (Pawn|Input|AddControllerPitchInput (.y ActionValue))))

(event Input|EnhancedActionEvents|EnhancedInputActionIA_SteerHovercraft
  (params (ActionValue :type Float%20%28double-precision%29) (ElapsedSeconds :type Float%20%28double-precision%29) (TriggeredSeconds :type Float%20%28double-precision%29) (InputAction :type Input%20Action%20Object%20Reference :default "/Game/Niels/Input/IA_SteerHovercraft.IA_SteerHovercraft"))
  (bind _returnvalue (Transformation|GetActorRotation))
  (bind _rotationspeed (Variables|Default|GetRotationSpeed))
  (bind _yaw (Math|Rotator|BreakRotator _returnvalue))
  (bind _returnvalue_2 (* ActionValue _rotationspeed))
  (bind _returnvalue_3 (+ _yaw _returnvalue_2))
  (:Triggered
    (if (>= _returnvalue_3 359.0)
      (Transformation|SetActorRotation "0, 0, 0")
      (else
        (Transformation|SetActorRotation (Math|Rotator|MakeRotator 0.0 0.0 _returnvalue_3))))))

(event Input|EnhancedActionEvents|EnhancedInputActionIA_Acceleration
  (params (ActionValue :type Float%20%28double-precision%29) (ElapsedSeconds :type Float%20%28double-precision%29) (TriggeredSeconds :type Float%20%28double-precision%29) (InputAction :type Input%20Action%20Object%20Reference :default "/Game/Niels/Input/IA_Acceleration.IA_Acceleration"))
  (bind _returnvalue (Transformation|GetActorRotation))
  (bind (_roll _pitch _yaw) (Math|Rotator|BreakRotator _returnvalue))
  (:Triggered
    (Pawn|Input|AddMovementInput (Math|Vector|GetForwardVector (Math|Rotator|MakeRotator _roll 0.0 _yaw)) 1.0 false)))

(event EventBeginPlay
  (bind _asplayer_controller (Utilities|Casting|CastToPlayerController (Pawn|GetController)))
  (Utilities|IsValid (PlayerController|LocalPlayerSubsystems|GetEnhancedInputLocalPlayerSubsystem _asplayer_controller)
    (:Is%20Valid
      (Input|AddMappingContext (PlayerController|LocalPlayerSubsystems|GetEnhancedInputLocalPlayerSubsystem _asplayer_controller) "/Game/Niels/Input/IMC_ControllerInput.IMC_ControllerInput" 0 "(bIgnoreAllPressedKeysUntilRelease=True,bForceImmediately=False)"))))

(fn ConstructionScript)