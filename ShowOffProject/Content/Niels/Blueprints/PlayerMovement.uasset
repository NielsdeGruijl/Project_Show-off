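; Player movement component that drives a hovercraft PlayerPawn through its FloatingPawnMovement, using tuning values copied from the pawn.
; Enhanced Input handles throttle, reverse by flipping acceleration direction, yaw steering, and drifting that swaps turn rate and TurningBoost above a minimum horizontal speed.
; Tick adds gravity to velocity and lerps the spring arm behind the craft unless the camera is being rotated, with a delay after release.
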(event Input|EnhancedActionEvents|EnhancedInputActionIA_Drifting
  (params (ActionValue :type Float%20%28double-precision%29) (ElapsedSeconds :type Float%20%28double-precision%29) (TriggeredSeconds :type Float%20%28double-precision%29) (InputAction :type Input%20Action%20Object%20Reference :default "/Game/Niels/Input/IA_Drifting.IA_Drifting"))
  (bind _playerpawn (Variables|Default|GetPlayerPawn))
  (bind _returnvalue (Transformation|GetVelocity _playerpawn))
  (bind (_x _y) (Math|Vector|BreakVector _returnvalue))
  ;[1 1 1] Drifting
  (:Triggered
    (if (>= (Math|Vector|VectorLength (Math|Vector|MakeVector _x _y 0.0)) 1.5e+02)
      (Variables|/Script/Engine.FloatingPawnMovement|SetTurningBoost (Variables|Default|GetPawnMovement) (Variables|Default|GetDriftTurningBoost))
      (Variables|Default|SetSteeringMultiplier (Variables|Default|GetDriftRotSpeed))))
  (:Completed
    (Variables|/Script/Engine.FloatingPawnMovement|SetTurningBoost (Variables|Default|GetPawnMovement) (Variables|Default|GetTurningBoost))
    (Variables|Default|SetSteeringMultiplier (Variables|Default|GetRotationSpeed))))

(event Input|EnhancedActionEvents|EnhancedInputActionIA_Reverse
  (params (ActionValue :type Float%20%28double-precision%29) (ElapsedSeconds :type Float%20%28double-precision%29) (TriggeredSeconds :type Float%20%28double-precision%29) (InputAction :type Input%20Action%20Object%20Reference :default "/Game/Niels/Input/IA_Reverse.IA_Reverse"))
  ;[1 1 1] Reverse
  (:Triggered
    (if (> -0.8 ActionValue)
      (Variables|Default|SetAccelerationDir -1.0)
      (else
        (Variables|Default|SetAccelerationDir 1.0))))
  (:Completed
    (Variables|Default|SetAccelerationDir 1.0)))

(event Input|EnhancedActionEvents|EnhancedInputActionIA_RotateCamera
  (params (ActionValue :type Float%20%28double-precision%29) (ElapsedSeconds :type Float%20%28double-precision%29) (TriggeredSeconds :type Float%20%28double-precision%29) (InputAction :type Input%20Action%20Object%20Reference :default "/Game/Niels/Input/IA_RotateCamera.IA_RotateCamera"))
  (bind _playerpawn (Variables|Default|GetPlayerPawn))
  (bind _springarm (Variables|/Game/Niels/PlayerPawn.PlayerPawn_C|GetSpringArm _playerpawn))
  ;[1 1 1] Rotate Camera
  (:Triggered
    (Variables|Default|SetControllingCamera true)
    (Transformation|SetWorldRotation _springarm (Math|Rotator|MakeRotator 0.0 0.0 (+ (* ActionValue (Variables|Default|GetCameraRotSpeed)) (.Yaw (Math|Rotator|BreakRotator (Transformation|GetWorldRotation _springarm))))) false false))
  (:Completed
    (Utilities|FlowControl|Delay 1.0)
    (Variables|Default|SetControllingCamera false)))

(event Input|EnhancedActionEvents|EnhancedInputActionIA_SteerHovercraft
  (params (ActionValue :type Float%20%28double-precision%29) (ElapsedSeconds :type Float%20%28double-precision%29) (TriggeredSeconds :type Float%20%28double-precision%29) (InputAction :type Input%20Action%20Object%20Reference :default "/Game/Niels/Input/IA_SteerHovercraft.IA_SteerHovercraft"))
  ;[1 1 1] Steering
  (:Triggered
    (Transformation|AddRelativeRotation (Variables|/Script/Engine.Actor|GetRootComponent (Variables|Default|GetPlayerPawn)) (Math|Rotator|MakeRotator 0.0 0.0 (* ActionValue (Variables|Default|GetSteeringMultiplier) (Utilities|Time|GetWorldDeltaSeconds))) false false)
    (Variables|/Game/Niels/PlayerPawn.PlayerPawn_C|SetSteeringInput (Variables|Default|GetPlayerPawn) ActionValue))
  (:Completed
    (Variables|/Game/Niels/PlayerPawn.PlayerPawn_C|SetSteeringInput (Variables|Default|GetPlayerPawn) 0.0)))

(event Input|EnhancedActionEvents|EnhancedInputActionIA_Acceleration
  (params (ActionValue :type Float%20%28double-precision%29) (ElapsedSeconds :type Float%20%28double-precision%29) (TriggeredSeconds :type Float%20%28double-precision%29) (InputAction :type Input%20Action%20Object%20Reference :default "/Game/Niels/Input/IA_Acceleration.IA_Acceleration"))
  (bind _playerpawn (Variables|Default|GetPlayerPawn))
  (bind _playerpawn_2 (Variables|Default|GetPlayerPawn))
  (bind _returnvalue (Transformation|GetActorRotation _playerpawn_2))
  (bind _floatingpawnmovement (Variables|/Game/Niels/PlayerPawn.PlayerPawn_C|GetFloatingPawnMovement _playerpawn))
  (bind (_roll _pitch _yaw) (Math|Rotator|BreakRotator _returnvalue))
  ;[1 1 1] Accelerating
  (:Triggered
    (Class|PawnMovementComponent|AddInputVector _floatingpawnmovement (* (Math|Vector|GetForwardVector (Math|Rotator|MakeRotator _roll 0.0 _yaw)) ActionValue (Variables|Default|GetAcceleration) (Variables|Default|GetAccelerationDir)) false)
    (Variables|/Script/Engine.FloatingPawnMovement|SetMaxSpeed _floatingpawnmovement (* ActionValue (Variables|/Game/Niels/PlayerPawn.PlayerPawn_C|GetMaxSpeed (Variables|Default|GetPlayerPawn))))))

(event EventTick
  (params (DeltaSeconds :type Float%20%28single-precision%29))
  ;[1 1 1] Gravity
  (if (Variables|/Game/Niels/PlayerPawn.PlayerPawn_C|GetEnableGravity (Variables|Default|GetPlayerPawn))
    (Variables|/Script/Engine.MovementComponent|SetVelocity (Variables|Default|GetPawnMovement) (+ (Variables|/Script/Engine.MovementComponent|GetVelocity (Variables|Default|GetPawnMovement)) (* DeltaSeconds (Variables|Default|GetGravity)))))
  (if (>= 5.0 (.Z (Math|Vector|BreakVector "0, 0, 0")))
    (Variables|/Game/Niels/PlayerPawn.PlayerPawn_C|SetEnableGravity (Variables|Default|GetPlayerPawn) true))
  (if (not (Variables|Default|GetControllingCamera))
    (CallFunction|ResetCameraPos)))

(event EventBeginPlay
  ;[1 1 1] Setup Variables
  (Utilities|FlowControl|Sequence
    (:then_0
      (bind _asplayer_pawn (Utilities|Casting|CastToPlayerPawn (Components|GetOwner)))
      (bind _output_get (Variables|Default|SetPlayerPawn _asplayer_pawn))
      (Variables|Default|SetPawnMovement (Variables|/Game/Niels/PlayerPawn.PlayerPawn_C|GetFloatingPawnMovement _output_get)))
    (:then_1
      (Variables|/Script/Engine.FloatingPawnMovement|SetMaxSpeed (Variables|/Game/Niels/PlayerPawn.PlayerPawn_C|GetFloatingPawnMovement (Variables|Default|GetPlayerPawn)) (Variables|/Game/Niels/PlayerPawn.PlayerPawn_C|GetMaxSpeed (Variables|Default|GetPlayerPawn)))
      (Variables|Default|SetRotationSpeed (Variables|/Game/Niels/PlayerPawn.PlayerPawn_C|GetRotationSpeed (Variables|Default|GetPlayerPawn)))
      (Variables|Default|SetDriftRotSpeed (Variables|/Game/Niels/PlayerPawn.PlayerPawn_C|GetDriftRotSpeed (Variables|Default|GetPlayerPawn)))
      (Variables|Default|SetTurningBoost (Variables|/Game/Niels/PlayerPawn.PlayerPawn_C|GetTurningBoost (Variables|Default|GetPlayerPawn)))
      (Variables|Default|SetDriftTurningBoost (Variables|/Game/Niels/PlayerPawn.PlayerPawn_C|GetDriftTurningBoost (Variables|Default|GetPlayerPawn)))
      (Variables|Default|SetCameraRotSpeed (Variables|/Game/Niels/PlayerPawn.PlayerPawn_C|GetCameraRotSpeed (Variables|Default|GetPlayerPawn)))
      (Variables|Default|SetSteeringInput 0.0)
      (Variables|Default|SetSteeringMultiplier (Variables|Default|GetRotationSpeed))
      (Variables|Default|SetAccelerationDir 1.0))))

(fn ResetCameraPos
  (bind _playerpawn (Variables|Default|GetPlayerPawn))
  (bind _playerpawn_2 (Variables|Default|GetPlayerPawn))
  (bind _returnvalue (Transformation|GetActorRotation _playerpawn_2))
  (bind _springarm (Variables|/Game/Niels/PlayerPawn.PlayerPawn_C|GetSpringArm _playerpawn))
  (bind (_roll _pitch _yaw) (Math|Rotator|BreakRotator _returnvalue))
  (Transformation|SetWorldRotation _springarm (Math|Rotator|Lerp(Rotator) (Transformation|GetWorldRotation _springarm) (Math|Rotator|MakeRotator _roll _pitch _yaw) 0.1 true) false false))