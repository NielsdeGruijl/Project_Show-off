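; Component that drives the cosmetic animation and speed feedback for the player's airboat pawn, caching its parts on BeginPlay.
; Every tick, horizontal speed relative to MaxSpeed sets camera FOV and camera shake scale and spins the fan.
; FOV snaps wider but eases back when narrowing by a degree or more.
; Both wings lerp their yaw opposite the steering input, both reading the first wing's current yaw.
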(event EventBeginPlay
  (Utilities|FlowControl|Sequence
    (:then_0
      (bind _asplayer_pawn (Utilities|Casting|CastToPlayerPawn (Components|GetOwner)))
      (Variables|Default|SetPlayerPawn _asplayer_pawn))
    (:then_1
      (Variables|Default|SetCamera (Variables|/Game/Niels/PlayerPawn.PlayerPawn_C|GetCamera (Variables|Default|GetPlayerPawn)))
      (Variables|Default|SetmaxSpeed (Variables|/Game/Niels/PlayerPawn.PlayerPawn_C|GetMaxSpeed (Variables|Default|GetPlayerPawn)))
      (Variables|Default|SetFanRotationSpeed (Variables|/Game/Niels/PlayerPawn.PlayerPawn_C|GetFanRotationSpeed (Variables|Default|GetPlayerPawn)))
      (Variables|Default|SetWingRotationSpeed (Variables|/Game/Niels/PlayerPawn.PlayerPawn_C|GetWingRotationSpeed (Variables|Default|GetPlayerPawn)))
      (Variables|Default|SetWing (Variables|/Game/Niels/PlayerPawn.PlayerPawn_C|Getwings (Variables|Default|GetPlayerPawn)))
      (Variables|Default|SetWing1 (Variables|/Game/Niels/PlayerPawn.PlayerPawn_C|Getwings1 (Variables|Default|GetPlayerPawn))))))

(event EventTick
  (params (DeltaSeconds :type Float%20%28single-precision%29))
  (CallFunction|ApplyVisualEffects)
  (CallFunction|AnimateFan)
  (CallFunction|AnimateWings))

(fn ApplyVisualEffects
  (bind _playerpawn (Variables|Default|GetPlayerPawn))
  (bind _playerpawn_2 (Variables|Default|GetPlayerPawn))
  (bind _camera (Variables|Default|GetCamera))
  (bind _deltafov (Variables|Default|GetDeltaFOV))
  (bind _floatingpawnmovement (Variables|/Game/Niels/PlayerPawn.PlayerPawn_C|GetFloatingPawnMovement _playerpawn_2))
  (bind _fieldofview (Variables|/Script/Engine.CameraComponent|GetFieldOfView _camera))
  (bind _maxspeed (Variables|/Game/Niels/PlayerPawn.PlayerPawn_C|GetMaxSpeed _playerpawn))
  (bind _velocity (Variables|/Script/Engine.MovementComponent|GetVelocity _floatingpawnmovement))
  (bind (_x _y) (Math|Vector|BreakVector _velocity))
  (bind _returnvalue (Math|Vector|MakeVector _x _y 0.0))
  (bind _returnvalue_2 (Math|Vector|VectorLength _returnvalue))
  (bind _returnvalue_3 (/ _returnvalue_2 _maxspeed))
  (bind _returnvalue_4 (* _returnvalue_3 _deltafov))
  (bind _returnvalue_5 (+ _returnvalue_4 9e+01))
  (Utilities|FlowControl|Sequence
    (:then_0
      (if (>= (- _fieldofview _returnvalue_5) 1.0)
        (Camera|SetFieldOfView (Variables|Default|GetCamera) (Math|Float|Lerp _fieldofview _returnvalue_5 0.2))
        (else
          (Camera|SetFieldOfView (Variables|Default|GetCamera) _returnvalue_5))))
    (:then_1
      (CameraShakes|StartCameraShake (Variables|/Game/Niels/PlayerPawn.PlayerPawn_C|GetCameraShakeSource (Variables|Default|GetPlayerPawn)) "/Game/Niels/Blueprints/MyShakeBase.MyShakeBase_C" _returnvalue_4 "CameraLocal" "0, 0, 0"))))

(fn AnimateFan
  (bind _playerpawn (Variables|Default|GetPlayerPawn))
  (bind _returnvalue (Transformation|GetVelocity _playerpawn))
  (bind (_x _y) (Math|Vector|BreakVector _returnvalue))
  (Transformation|AddRelativeRotation (Variables|/Game/Niels/PlayerPawn.PlayerPawn_C|GetSM_airboat_fan (Variables|Default|GetPlayerPawn)) (Math|Rotator|MakeRotator (* (/ (Math|Vector|VectorLength (Math|Vector|MakeVector _x _y 0.0)) (Variables|/Game/Niels/PlayerPawn.PlayerPawn_C|GetMaxSpeed (Variables|Default|GetPlayerPawn))) (Variables|Default|GetFanRotationSpeed)) 0.0 0.0) false false))

(fn AnimateWings
  (bind _playerpawn (Variables|Default|GetPlayerPawn))
  (bind _wing (Variables|Default|GetWing))
  (bind _wing_2 (Variables|Default|GetWing))
  (bind _wingrotationspeed (Variables|Default|GetWingRotationSpeed))
  (bind _wingrotationspeed_2 (Variables|Default|GetWingRotationSpeed))
  (bind _wing_3 (Variables|Default|GetWing))
  (bind _wing1 (Variables|Default|GetWing1))
  (bind _playerpawn_2 (Variables|Default|GetPlayerPawn))
  (bind _relativerotation (Variables|/Script/Engine.SceneComponent|GetRelativeRotation _wing))
  (bind _relativerotation_2 (Variables|/Script/Engine.SceneComponent|GetRelativeRotation _wing_2))
  (bind _steeringinput (Variables|/Game/Niels/PlayerPawn.PlayerPawn_C|GetSteeringInput _playerpawn_2))
  (bind _wingrotation (Variables|/Game/Niels/PlayerPawn.PlayerPawn_C|GetWingRotation _playerpawn))
  (bind _yaw (Math|Rotator|BreakRotator _relativerotation))
  (bind _yaw_2 (Math|Rotator|BreakRotator _relativerotation_2))
  (bind _returnvalue (* _steeringinput -1.0))
  (bind _returnvalue_2 (Math|Float|Lerp _yaw 0.0 _wingrotationspeed_2))
  (bind _returnvalue_3 (* _returnvalue _wingrotation))
  (bind _returnvalue_4 (Math|Float|Lerp _yaw_2 _returnvalue_3 _wingrotationspeed))
  (bind _returnvalue_5 (Math|Rotator|MakeRotator 0.0 0.0 _returnvalue_2))
  (bind _returnvalue_6 (Math|Rotator|MakeRotator 0.0 0.0 _returnvalue_4))
  (if (== _steeringinput 0.0)
    (Transformation|SetRelativeRotation _wing_3 _returnvalue_5 false false)
    (Transformation|SetRelativeRotation _wing1 _returnvalue_5 false false)
    (else
      (Transformation|SetRelativeRotation _wing_3 _returnvalue_6 false false)
      (Transformation|SetRelativeRotation _wing1 _returnvalue_6 false false))))