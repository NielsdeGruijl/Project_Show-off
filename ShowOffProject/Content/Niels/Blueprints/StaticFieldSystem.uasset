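; Field System actor that sets the Chaos physics dynamic state of objects inside its box volume, likely to anchor destructibles as the name suggests.
; Shortly after BeginPlay, it adds a single dynamic-state field command to its Field System component.
; The command feeds a uniform integer from ObjectState through a culling field, using a no-falloff box field from the Box component's world transform to limit it to the inside.
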(event EventBeginPlay
  (Utilities|FlowControl|Delay 0.2)
  (Class|FieldSystemComponent|AddFieldCommand (Variables|Field|GetFieldSystemComponent) false "Field_DynamicState" 0 (Field|SetCullingField (Variables|Default|GetCullingField) (Field|SetBoxFalloff (Variables|Default|GetBoxFalloff) 1.0 0.0 1.0 0.0 (Transformation|GetWorldTransform (Variables|Default|GetBox)) "Field_FallOff_None") (Field|SetUniformInteger (Variables|Default|GetUniformInteger) (Math|Conversions|ToInteger(Byte) (Variables|Default|GetObject%20state))) "Field_Culling_Inside")))

(fn ConstructionScript)