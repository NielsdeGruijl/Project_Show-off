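; Sound manager that gives its owning PlayerPawn per-player voice reactions, winning sounds and boat acceleration audio.
; PlaySound and PlayWinningSound choose random 2D clips from Player 1 or Player 2 arrays by player index.
; Bad sounds are followed after a delay by a fixed "too easy" taunt.
; A looping-style acceleration sound spawns muted at BeginPlay, and Tick scales its volume by horizontal speed relative to MaxSpeed.
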(event Custom|PlaySound
  (params (IsGoodSound :type Boolean))
  (bind _player1goodsounds (Variables|Default|GetPlayer1GoodSounds))
  (bind _player2goodsounds (Variables|Default|GetPlayer2GoodSounds))
  (bind _player1badsounds (Variables|Default|GetPlayer1BadSounds))
  (bind _player2badsounds (Variables|Default|GetPlayer2BadSounds))
  (bind _asplayer_pawn (Utilities|Casting|CastToPlayerPawn (Components|GetOwner))
    (:then
      (if (== (Variables|/Game/Niels/PlayerPawn.PlayerPawn_C|GetPlayerIndex _asplayer_pawn) 0)
        (if IsGoodSound
          (Audio|PlaySound2D (Utilities|Array|Get(acopy) _player1goodsounds (Math|Random|RandomInteger (Utilities|Array|Length _player1goodsounds))) 1.0 1.0 0.0 0 0)
          (else
            (Audio|PlaySound2D (Utilities|Array|Get(acopy) _player1badsounds (Math|Random|RandomInteger (Utilities|Array|Length _player1badsounds))) 1.0 1.0 0.0 0 0)
            (Utilities|FlowControl|Delay 4.5)
            (Audio|PlaySound2D "/Game/Kai/Audio/Audio_files/Voice_Lines/Els/els_too_easy2.els_too_easy2" 1.0 1.0 0.0 0 0)))
        (elif IsGoodSound
          (Audio|PlaySound2D (Utilities|Array|Get(acopy) _player2goodsounds (Math|Random|RandomInteger (Utilities|Array|Length _player2goodsounds))) 1.0 1.0 0.0 0 0)
          (else
            (Audio|PlaySound2D (Utilities|Array|Get(acopy) _player2badsounds (Math|Random|RandomInteger (Utilities|Array|Length _player2badsounds))) 1.0 1.0 0.0 0 0)
            (Utilities|FlowControl|Delay 4.0)
            (Audio|PlaySound2D "/Game/Kai/Audio/Audio_files/Voice_Lines/Menji/menji_too_easy1.menji_too_easy1" 1.0 1.0 0.0 0 0)))))
    (:CastFailed
      (Development|PrintString "Wrong cast in soundmanager"))))

(event Custom|Play%20Winning%20Sound
  (params (PlayerIndex :type Integer))
  (bind _player1winningsounds (Variables|Default|GetPlayer1WinningSounds))
  (bind _player2winningsounds (Variables|Default|GetPlayer2WinningSounds))
  (if (== PlayerIndex 0)
    (Audio|PlaySound2D (Utilities|Array|Get(acopy) _player1winningsounds (Math|Random|RandomInteger (Utilities|Array|Length _player1winningsounds))) 1.0 1.0 0.0 0 0)
    (else
      (Audio|PlaySound2D (Utilities|Array|Get(acopy) _player2winningsounds (Math|Random|RandomInteger (Utilities|Array|Length _player2winningsounds))) 1.0 1.0 0.0 0 0))))

(event EventBeginPlay
  (bind _returnvalue (Audio|SpawnSound2D "/Game/Kai/Audio/Metasounds/Boat_Acceleration.Boat_Acceleration" 1.0 1.0 0.0 0))
  (bind _output_get (Variables|Default|SetSpawnedAccelerationSound _returnvalue))
  (Audio|Components|Audio|SetVolumeMultiplier _output_get 0.0 :!class /Script/Engine.AudioComponent))

(event EventTick
  (params (DeltaSeconds :type Float%20%28single-precision%29))
  (bind _asplayer_pawn (Utilities|Casting|CastToPlayerPawn (Components|GetOwner)))
  (Audio|Components|Audio|SetVolumeMultiplier (Variables|Default|GetSpawnedAccelerationSound) (* (/ (Math|Vector|VectorLength (Math|Vector|MakeVector (.X (Math|Vector|BreakVector (Transformation|GetVelocity _asplayer_pawn))) (.Y (Math|Vector|BreakVector (Transformation|GetVelocity _asplayer_pawn))) 0.0)) (Variables|/Game/Niels/PlayerPawn.PlayerPawn_C|GetMaxSpeed _asplayer_pawn)) 3.0) :!class /Script/Engine.AudioComponent))