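; Pawn component that runs potion use in a two-player game.
; TriggerPotionUse applies the held potion, empties the inventory and undoes the effect after a fixed delay.
; Speed and Immunity buff the user, while Slow Down and Blindness call the opponent's potion manager, which ignores them if immune.
; Effects change movement speed, particles, a hallucination post-process blendable or a mud HUD overlay, tracked by one ActivePotionEffect per pawn.
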(event Custom|Trigger%20Potion%20Use
  (bind _asplayer_pawn (Utilities|Casting|CastToPlayerPawn (Components|GetOwner)))
  (Development|PrintString "Trying to use potion")
  (if (Utilities|Enum|NotEqual(Enum) (Variables|/Game/Niels/PlayerPawn.PlayerPawn_C|GetCurrentHoldingPotion _asplayer_pawn) "None")
    (Audio|PlaySound2D "/Game/Kai/Audio/Metasounds/Potion_throw.Potion_throw" 1.0 1.0 0.0 0 0)
    (switch string (Variables|/Game/Niels/PlayerPawn.PlayerPawn_C|GetCurrentHoldingPotion _asplayer_pawn)
      (:SpeedPotion
        (if (Utilities|Enum|NotEqual(Enum) (Variables|/Game/Niels/PlayerPawn.PlayerPawn_C|GetActivePotionEffect _asplayer_pawn) "Immunity")
          (Default|PlaySound (Variables|/Game/Niels/PlayerPawn.PlayerPawn_C|GetBP_SoundManager _asplayer_pawn) true)
          (CallFunction|ResetPotionEffects)
          (CallFunction|UsePotion)
          (Utilities|FlowControl|Delay 7.0)
          (CallFunction|ResetPotionEffects :!label _label)
          (else
            (Default|RemoveAllPotions (Variables|/Game/Niels/PlayerPawn.PlayerPawn_C|GetBPC_Inventory _asplayer_pawn) :!label _label_2))))
      (:SlowDownPotion
        (CallFunction|UsePotion)
        (Utilities|FlowControl|Delay 7.0)
        (CallFunction|ResetAttackPotionEffects "SlowDown" (Variables|/Game/Niels/PlayerPawn.PlayerPawn_C|GetPlayerIndex _asplayer_pawn)))
      (:ImmunityPotion
        (if true
          (Default|PlaySound (Variables|/Game/Niels/PlayerPawn.PlayerPawn_C|GetBP_SoundManager _asplayer_pawn) true)
          (CallFunction|ResetPotionEffects)
          (CallFunction|UsePotion)
          (Utilities|FlowControl|Delay 2e+01)
          (goto _label)
          (else
            (goto _label_2))))
      (:BlindnessPotion
        (CallFunction|UsePotion)
        (Utilities|FlowControl|Delay 7.0)
        (CallFunction|ResetAttackPotionEffects "Blindness" (Variables|/Game/Niels/PlayerPawn.PlayerPawn_C|GetPlayerIndex _asplayer_pawn))))
    (else
      (Development|PrintString "Doesn't have a potion to use"))))

(fn UsePotion
  (bind _asplayer_pawn (Utilities|Casting|CastToPlayerPawn (Components|GetOwner)))
  (switch string (Variables|/Game/Niels/PlayerPawn.PlayerPawn_C|GetCurrentHoldingPotion _asplayer_pawn)
    (:SpeedPotion
      (CallFunction|ExecuteSpeedPotion))
    (:SlowDownPotion
      (CallFunction|ExecuteSlowDownPotion true))
    (:ImmunityPotion
      (CallFunction|ExecuteImmunityPotion))
    (:BlindnessPotion
      (CallFunction|ExecuteBlindnessPotion true)))
  (Default|RemoveAllPotions (Variables|/Game/Niels/PlayerPawn.PlayerPawn_C|GetBPC_Inventory _asplayer_pawn)))

(fn ExecuteSpeedPotion
  (bind _asplayer_pawn (Utilities|Casting|CastToPlayerPawn (Components|GetOwner)))
  (Variables|/Script/Engine.FloatingPawnMovement|SetMaxSpeed (Variables|/Game/Niels/PlayerPawn.PlayerPawn_C|GetFloatingPawnMovement _asplayer_pawn) (+ (Class|MovementComponent|GetMaxSpeed (Variables|/Game/Niels/PlayerPawn.PlayerPawn_C|GetFloatingPawnMovement _asplayer_pawn)) 1.5e+02))
  (Components|Activation|SetActive (Variables|/Game/Niels/PlayerPawn.PlayerPawn_C|GetSpeedLines _asplayer_pawn) true false)
  (Variables|/Game/Niels/PlayerPawn.PlayerPawn_C|SetActivePotionEffect _asplayer_pawn "Speed"))

(fn ExecuteBlindnessPotion
  (params (IsExecuter :type Boolean))
  (bind _asplayer_pawn (Utilities|Casting|CastToPlayerPawn (Components|GetOwner)))
  (if IsExecuter
    (if (== (Variables|/Game/Niels/PlayerPawn.PlayerPawn_C|GetPlayerIndex _asplayer_pawn) 0)
      (bind _asplayer_pawn_2 (Utilities|Casting|CastToPlayerPawn (Game|Player|GetPlayerPawn 1)))
      (Default|PlaySound (Variables|/Game/Niels/PlayerPawn.PlayerPawn_C|GetBP_SoundManager _asplayer_pawn_2) false)
      (CallFunction|ExecuteBlindnessPotion (Variables|/Game/Niels/PlayerPawn.PlayerPawn_C|GetBP_PotionManager _asplayer_pawn_2) false)
      (else
        (bind _asplayer_pawn_3 (Utilities|Casting|CastToPlayerPawn (Game|Player|GetPlayerPawn 0)))
        (Default|PlaySound (Variables|/Game/Niels/PlayerPawn.PlayerPawn_C|GetBP_SoundManager _asplayer_pawn_3) false)
        (CallFunction|ExecuteBlindnessPotion (Variables|/Game/Niels/PlayerPawn.PlayerPawn_C|GetBP_PotionManager _asplayer_pawn_3) false)))
    (elif (not (Utilities|Enum|Equal(Enum) (Variables|/Game/Niels/PlayerPawn.PlayerPawn_C|GetActivePotionEffect _asplayer_pawn) "Immunity"))
      (CallFunction|ResetPotionEffects)
      (bind _asliam_game_mode (Utilities|Casting|CastToLiam_GameMode (Game|GetGameMode)))
      (if (== (Variables|/Game/Niels/PlayerPawn.PlayerPawn_C|GetPlayerIndex _asplayer_pawn) 0)
        (Default|ChangeMudVisibility (Variables|/Game/Liam/Liam_GameMode.Liam_GameMode_C|GetInventory_PL1 _asliam_game_mode) true)
        (else
          (Default|ChangeMudVisibility (Variables|/Game/Liam/Liam_GameMode.Liam_GameMode_C|GetInventory_PL2 _asliam_game_mode) true)))
      (Variables|/Game/Niels/PlayerPawn.PlayerPawn_C|SetActivePotionEffect _asplayer_pawn "Blindness"))))

(fn ExecuteImmunityPotion
  (bind _asplayer_pawn (Utilities|Casting|CastToPlayerPawn (Components|GetOwner)))
  (Variables|/Game/Niels/PlayerPawn.PlayerPawn_C|SetActivePotionEffect _asplayer_pawn "Immunity")
  (Components|Activation|SetActive (Variables|/Game/Niels/PlayerPawn.PlayerPawn_C|GetParticles _asplayer_pawn) true false))

(fn ExecuteSlowDownPotion
  (params (IsExecuter :type Boolean))
  (bind _asplayer_pawn (Utilities|Casting|CastToPlayerPawn (Components|GetOwner)))
  (if IsExecuter
    (if (== (Variables|/Game/Niels/PlayerPawn.PlayerPawn_C|GetPlayerIndex _asplayer_pawn) 0)
      (bind _asplayer_pawn_2 (Utilities|Casting|CastToPlayerPawn (Game|Player|GetPlayerPawn 1)))
      (Default|PlaySound (Variables|/Game/Niels/PlayerPawn.PlayerPawn_C|GetBP_SoundManager _asplayer_pawn_2) false)
      (CallFunction|ExecuteSlowDownPotion (Variables|/Game/Niels/PlayerPawn.PlayerPawn_C|GetBP_PotionManager _asplayer_pawn_2) false)
      (else
        (bind _asplayer_pawn_3 (Utilities|Casting|CastToPlayerPawn (Game|Player|GetPlayerPawn 0)))
        (Default|PlaySound (Variables|/Game/Niels/PlayerPawn.PlayerPawn_C|GetBP_SoundManager _asplayer_pawn_3) false)
        (CallFunction|ExecuteSlowDownPotion (Variables|/Game/Niels/PlayerPawn.PlayerPawn_C|GetBP_PotionManager _asplayer_pawn_3) false)))
    (elif (not (Utilities|Enum|Equal(Enum) (Variables|/Game/Niels/PlayerPawn.PlayerPawn_C|GetActivePotionEffect _asplayer_pawn) "Immunity"))
      (CallFunction|ResetPotionEffects)
      (bind _returnvalue (Rendering|Material|CreateDynamicMaterialInstance "/Game/Liam/Material/M_Hallucination.M_Hallucination" "None" "None" :!class /Script/Engine.KismetMaterialLibrary))
      (Rendering|AddorUpdateBlendable (Variables|/Game/Niels/PlayerPawn.PlayerPawn_C|GetCamera _asplayer_pawn) _returnvalue 1.0 :!class /Script/Engine.CameraComponent)
      (Variables|/Game/Niels/PlayerPawn.PlayerPawn_C|SetActiveDynamicMaterial _asplayer_pawn _returnvalue)
      (Variables|/Script/Engine.FloatingPawnMovement|SetMaxSpeed (Variables|/Game/Niels/PlayerPawn.PlayerPawn_C|GetFloatingPawnMovement _asplayer_pawn) (- (Class|MovementComponent|GetMaxSpeed (Variables|/Game/Niels/PlayerPawn.PlayerPawn_C|GetFloatingPawnMovement _asplayer_pawn)) 1.5e+02))
      (Variables|/Game/Niels/PlayerPawn.PlayerPawn_C|SetActivePotionEffect _asplayer_pawn "SlowDown"))))

(fn ResetPotionEffects
  (bind _asplayer_pawn (Utilities|Casting|CastToPlayerPawn (Components|GetOwner)))
  (switch string (Variables|/Game/Niels/PlayerPawn.PlayerPawn_C|GetActivePotionEffect _asplayer_pawn)
    (:Speed
      (Variables|/Script/Engine.FloatingPawnMovement|SetMaxSpeed (Variables|/Game/Niels/PlayerPawn.PlayerPawn_C|GetFloatingPawnMovement _asplayer_pawn) (- (Class|MovementComponent|GetMaxSpeed (Variables|/Game/Niels/PlayerPawn.PlayerPawn_C|GetFloatingPawnMovement _asplayer_pawn)) 1.5e+02))
      (Components|Activation|SetActive (Variables|/Game/Niels/PlayerPawn.PlayerPawn_C|GetSpeedLines _asplayer_pawn) false false)
      (Variables|/Game/Niels/PlayerPawn.PlayerPawn_C|SetActivePotionEffect _asplayer_pawn "None"))
    (:Immunity
      (Variables|/Game/Niels/PlayerPawn.PlayerPawn_C|SetActivePotionEffect _asplayer_pawn "None")
      (Components|Activation|SetActive (Variables|/Game/Niels/PlayerPawn.PlayerPawn_C|GetParticles _asplayer_pawn) false false))))

(fn ResetAttackPotionEffects
  (params (UsedPotion :type String) (PlayerIndex :type Integer))
  (bind _returnvalue (Game|GetGameMode))
  (switch string UsedPotion
    (:SlowDown
      (if (== PlayerIndex 0)
        (bind _asplayer_pawn (Utilities|Casting|CastToPlayerPawn (Game|Player|GetPlayerPawn 1)))
        (Class|CameraComponent|RemoveBlendable (Variables|/Game/Niels/PlayerPawn.PlayerPawn_C|GetCamera _asplayer_pawn) (Variables|/Game/Niels/PlayerPawn.PlayerPawn_C|GetActiveDynamicMaterial _asplayer_pawn))
        (Variables|/Game/Niels/PlayerPawn.PlayerPawn_C|SetActiveDynamicMaterial _asplayer_pawn 0)
        (Variables|/Script/Engine.FloatingPawnMovement|SetMaxSpeed (Variables|/Game/Niels/PlayerPawn.PlayerPawn_C|GetFloatingPawnMovement _asplayer_pawn) (+ (Class|MovementComponent|GetMaxSpeed (Variables|/Game/Niels/PlayerPawn.PlayerPawn_C|GetFloatingPawnMovement _asplayer_pawn)) 1.5e+02))
        (Variables|/Game/Niels/PlayerPawn.PlayerPawn_C|SetActivePotionEffect _asplayer_pawn "None")
        (else
          (bind _asplayer_pawn_2 (Utilities|Casting|CastToPlayerPawn (Game|Player|GetPlayerPawn 0)))
          (Class|CameraComponent|RemoveBlendable (Variables|/Game/Niels/PlayerPawn.PlayerPawn_C|GetCamera _asplayer_pawn_2) (Variables|/Game/Niels/PlayerPawn.PlayerPawn_C|GetActiveDynamicMaterial _asplayer_pawn_2))
          (Variables|/Game/Niels/PlayerPawn.PlayerPawn_C|SetActiveDynamicMaterial _asplayer_pawn_2 0)
          (Variables|/Script/Engine.FloatingPawnMovement|SetMaxSpeed (Variables|/Game/Niels/PlayerPawn.PlayerPawn_C|GetFloatingPawnMovement _asplayer_pawn_2) (+ (Class|MovementComponent|GetMaxSpeed (Variables|/Game/Niels/PlayerPawn.PlayerPawn_C|GetFloatingPawnMovement _asplayer_pawn_2)) 1.5e+02))
          (Variables|/Game/Niels/PlayerPawn.PlayerPawn_C|SetActivePotionEffect _asplayer_pawn_2 "None")
          (Development|PrintString "Hello"))))
    (:Blindness
      (if (== PlayerIndex 0)
        (bind _asplayer_pawn_3 (Utilities|Casting|CastToPlayerPawn (Game|Player|GetPlayerPawn 1)))
        (Variables|/Game/Niels/PlayerPawn.PlayerPawn_C|SetActivePotionEffect _asplayer_pawn_3 "None")
        (bind _asliam_game_mode (Utilities|Casting|CastToLiam_GameMode _returnvalue))
        (Default|ChangeMudVisibility (Variables|/Game/Liam/Liam_GameMode.Liam_GameMode_C|GetInventory_PL2 _asliam_game_mode) false)
        (else
          (bind _asplayer_pawn_4 (Utilities|Casting|CastToPlayerPawn (Game|Player|GetPlayerPawn 0)))
          (Variables|/Game/Niels/PlayerPawn.PlayerPawn_C|SetActivePotionEffect _asplayer_pawn_4 "None")
          (bind _asliam_game_mode_2 (Utilities|Casting|CastToLiam_GameMode _returnvalue))
          (Default|ChangeMudVisibility (Variables|/Game/Liam/Liam_GameMode.Liam_GameMode_C|GetInventory_PL1 _asliam_game_mode_2) false))))))

(fn SwitchPotionBook
  (bind _returnvalue (Game|GetGameMode))
  (bind _asplayer_pawn (Utilities|Casting|CastToPlayerPawn (Components|GetOwner)))
  (if (== (Variables|/Game/Niels/PlayerPawn.PlayerPawn_C|GetPlayerIndex _asplayer_pawn) 0)
    (bind _asliam_game_mode (Utilities|Casting|CastToLiam_GameMode _returnvalue))
    (Default|SwitchPotionBook (Variables|/Game/Liam/Liam_GameMode.Liam_GameMode_C|GetInventory_PL1 _asliam_game_mode))
    (elif (== (Variables|/Game/Niels/PlayerPawn.PlayerPawn_C|GetPlayerIndex _asplayer_pawn) 1)
      (bind _asliam_game_mode_2 (Utilities|Casting|CastToLiam_GameMode _returnvalue))
      (Default|SwitchPotionBook (Variables|/Game/Liam/Liam_GameMode.Liam_GameMode_C|GetInventory_PL2 _asliam_game_mode_2)))))