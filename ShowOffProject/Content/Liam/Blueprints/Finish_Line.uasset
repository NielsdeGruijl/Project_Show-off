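; Finish line actor that ends a two-player race when the first PlayerPawn overlaps its Box trigger.
; The winner's sound manager plays a winning sound, and a W_GameOver widget shows that player's one-based number.
; Both players' pawns are braked by zeroing max speed and setting high deceleration, and their controllers switch to UI-only input focused on the widget.
; A GameFinished flag blocks further triggers once the sequence completes.
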(event OnComponentBeginOverlap(Box)
  (params (OverlappedComponent :type Primitive%20Component%20Object%20Reference) (OtherActor :type Actor%20Object%20Reference) (OtherComp :type Primitive%20Component%20Object%20Reference) (OtherBodyIndex :type Integer) (bFromSweep :type Boolean) (SweepResult :type Hit%20Result%20Structure%20%28by%20ref%29))
  (if (not (Variables|Default|GetgameFinished))
    (bind _asplayer_pawn (Utilities|Casting|CastToPlayerPawn OtherActor))
    (bind _returnvalue (UserInterface|CreateWidget "/Game/Liam/Widgets/W_GameOver.W_GameOver_C" (Game|GetPlayerController 0)))
    (Default|PlayWinningSound (Variables|/Game/Niels/PlayerPawn.PlayerPawn_C|GetBP_SoundManager _asplayer_pawn) (Variables|/Game/Niels/PlayerPawn.PlayerPawn_C|GetPlayerIndex _asplayer_pawn))
    (bind _asplayer_pawn_2 (Utilities|Casting|CastToPlayerPawn (Game|Player|GetPlayerPawn 1)))
    (Variables|/Script/Engine.FloatingPawnMovement|SetMaxSpeed (Variables|/Game/Niels/PlayerPawn.PlayerPawn_C|GetFloatingPawnMovement _asplayer_pawn_2) 0.0)
    (Variables|/Script/Engine.FloatingPawnMovement|SetDeceleration (Variables|/Game/Niels/PlayerPawn.PlayerPawn_C|GetFloatingPawnMovement _asplayer_pawn_2) 1.5e+03)
    (Input|SetInputModeUIOnly (Game|GetPlayerController 1) _returnvalue "DoNotLock" false)
    (bind _asplayer_pawn_3 (Utilities|Casting|CastToPlayerPawn (Game|Player|GetPlayerPawn 0)))
    (Variables|/Script/Engine.FloatingPawnMovement|SetMaxSpeed (Variables|/Game/Niels/PlayerPawn.PlayerPawn_C|GetFloatingPawnMovement _asplayer_pawn_3) 0.0)
    (Variables|/Script/Engine.FloatingPawnMovement|SetDeceleration (Variables|/Game/Niels/PlayerPawn.PlayerPawn_C|GetFloatingPawnMovement _asplayer_pawn_3) 1.5e+03)
    (Input|SetInputModeUIOnly (Game|GetPlayerController 0) _returnvalue "DoNotLock" false)
    (Variables|/Game/Liam/Widgets/W_GameOver.W_GameOver_C|SetPlayerId _returnvalue (+ (Variables|/Game/Niels/PlayerPawn.PlayerPawn_C|GetPlayerIndex _asplayer_pawn) 1))
    (UserInterface|Viewport|AddtoViewport _returnvalue 0)
    (Class|CommonActivatableWidget|ActivateWidget _returnvalue)
    (Variables|Default|SetgameFinished true)))

(event EventBeginPlay)

(event Collision|EventActorBeginOverlap
  (params (OtherActor :type Actor%20Object%20Reference)))

(event EventTick
  (params (DeltaSeconds :type Float%20%28single-precision%29)))

(fn ConstructionScript)