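; Inventory component that stores a player's items by name and crafts Speed, Slow Down, Immunity and Blindness potions from them.
; Each potion has a hard-coded three-ingredient recipe; a successful craft consumes the ingredients and replaces any held potion.
; Adding items, crafting and clearing potions update the owner's inventory widget on Liam_GameMode, chosen by PlayerIndex for two players.
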(fn AddItemtoInventory
  (params (NewItem :type String%20%28by%20ref%29))
  (bind _returnvalue (Game|GetGameMode))
  (Utilities|Array|Add (Variables|Default|Getinventory) NewItem)
  (Development|PrintString "Item added to inventory")
  (bind _asniels_player_pawn (Utilities|Casting|CastTo (Components|GetOwner)))
  (if (== (Variables|Default|GetPlayerIndex _asniels_player_pawn) 0)
    (bind _asliam_game_mode (Utilities|Casting|CastToLiam_GameMode _returnvalue))
    (Default|AddItemtoListUI (Variables|/Game/Liam/Liam_GameMode.Liam_GameMode_C|GetInventory_PL1 _asliam_game_mode))
    (elif (== (Variables|Default|GetPlayerIndex _asniels_player_pawn) 1)
      (bind _asliam_game_mode_2 (Utilities|Casting|CastToLiam_GameMode _returnvalue))
      (Default|AddItemtoListUI (Variables|/Game/Liam/Liam_GameMode.Liam_GameMode_C|GetInventory_PL2 _asliam_game_mode_2)))))

(fn RemoveItemfromInventory
  (params (ItemToRemove :type String))
  (bind _returnvalue (Utilities|Array|RemoveItem (Variables|Default|Getinventory) ItemToRemove))
  (if _returnvalue
    (Development|PrintString "Item was removed successfully")
    (else
      (Development|PrintString "Couldn't find"))))

(fn CraftPotion
  (params (PotionToCraft :type String))
  (bind _returnvalue (Game|GetGameMode))
  (bind _returnvalue_2 (Utilities|String|Append PotionToCraft "Potion"))
  (bind _inventory (Variables|Default|Getinventory))
  (bind _inventory_2 (Variables|Default|Getinventory))
  (bind _inventory_3 (Variables|Default|Getinventory))
  (bind _inventory_4 (Variables|Default|Getinventory))
  (switch string PotionToCraft
    (:Speed
      (if (== (Utilities|Array|FindItem _inventory_2 "Fish") -1)
        (return false)
        (elif (== (Utilities|Array|FindItem _inventory_2 "Red Flower") -1)
          (return false)
          (elif (not (== (Utilities|Array|FindItem _inventory_2 "Seashell") -1))
            (CallFunction|RemoveAllPotions)
            (CallFunction|RemoveItemfromInventory "Fish")
            (CallFunction|RemoveItemfromInventory "Red Flower")
            (CallFunction|RemoveItemfromInventory "Seashell")
            (Utilities|Array|Add (Variables|Default|Getinventory) _returnvalue_2)
            (bind _asniels_player_pawn (Utilities|Casting|CastTo (Components|GetOwner) :!label _label))
            (if (== (Variables|Default|GetPlayerIndex _asniels_player_pawn) 0)
              (bind _asliam_game_mode (Utilities|Casting|CastToLiam_GameMode _returnvalue))
              (bind _output_get (Variables|Default|SetCurrentHoldingPotion _asniels_player_pawn _returnvalue_2))
              (Default|SwitchPotionBook (Variables|/Game/Liam/Liam_GameMode.Liam_GameMode_C|GetInventory_PL1 _asliam_game_mode))
              (Default|UpdateCurrentPotion (Variables|/Game/Liam/Liam_GameMode.Liam_GameMode_C|GetInventory_PL1 _asliam_game_mode))
              (Development|PrintString _output_get)
              (return true)
              (elif (== (Variables|Default|GetPlayerIndex _asniels_player_pawn) 1)
                (bind _asliam_game_mode_2 (Utilities|Casting|CastToLiam_GameMode _returnvalue))
                (Variables|Default|SetCurrentHoldingPotion _asniels_player_pawn _returnvalue_2)
                (Default|SwitchPotionBook (Variables|/Game/Liam/Liam_GameMode.Liam_GameMode_C|GetInventory_PL2 _asliam_game_mode_2))
                (Default|UpdateCurrentPotion (Variables|/Game/Liam/Liam_GameMode.Liam_GameMode_C|GetInventory_PL2 _asliam_game_mode_2))
                (return true)))))))
    (:SlowDown
      (if (== (Utilities|Array|FindItem _inventory_4 "Wood") -1)
        (return false)
        (elif (== (Utilities|Array|FindItem _inventory_4 "Leave") -1)
          (return false)
          (elif (not (== (Utilities|Array|FindItem _inventory_4 "Blue Flower") -1))
            (CallFunction|RemoveAllPotions)
            (CallFunction|RemoveItemfromInventory "Wood")
            (CallFunction|RemoveItemfromInventory "Leave")
            (CallFunction|RemoveItemfromInventory "Blue Flower")
            (Utilities|Array|Add (Variables|Default|Getinventory) _returnvalue_2)
            (goto _label)))))
    (:Immunity
      (if (== (Utilities|Array|FindItem _inventory_3 "Wood") -1)
        (return false)
        (elif (== (Utilities|Array|FindItem _inventory_3 "Leave") -1)
          (return false)
          (elif (not (== (Utilities|Array|FindItem _inventory_3 "Seashell") -1))
            (CallFunction|RemoveAllPotions)
            (CallFunction|RemoveItemfromInventory "Wood")
            (CallFunction|RemoveItemfromInventory "Leave")
            (CallFunction|RemoveItemfromInventory "Seashell")
            (Utilities|Array|Add (Variables|Default|Getinventory) _returnvalue_2)
            (goto _label)))))
    (:Blindness
      (if (== (Utilities|Array|FindItem _inventory "Leave") -1)
        (return false)
        (elif (== (Utilities|Array|FindItem _inventory "Red Flower") -1)
          (return false)
          (elif (not (== (Utilities|Array|FindItem _inventory "Blue Flower") -1))
            (CallFunction|RemoveAllPotions)
            (CallFunction|RemoveItemfromInventory "Leave")
            (CallFunction|RemoveItemfromInventory "Red Flower")
            (CallFunction|RemoveItemfromInventory "Blue Flower")
            (Utilities|Array|Add (Variables|Default|Getinventory) _returnvalue_2)
            (goto _label)))))))

(fn RemoveAllPotions
  (bind _returnvalue (Game|GetGameMode))
  (bind _inventory (Variables|Default|Getinventory))
  (bind _playerindex (Variables|Default|GetPlayerIndex))
  (if (== (Utilities|Array|FindItem _inventory "SpeedPotion") -1)
    _
    (else
      (Utilities|Array|RemoveItem _inventory "SpeedPotion")))
  (if (== (Utilities|Array|FindItem _inventory "SlowDownPotion") -1)
    _
    (else
      (Utilities|Array|RemoveItem _inventory "SlowDownPotion")))
  (if (== (Utilities|Array|FindItem _inventory "ImmunityPotion") -1)
    _
    (else
      (Utilities|Array|RemoveItem _inventory "ImmunityPotion")))
  (if (== (Utilities|Array|FindItem _inventory "BlindnessPotion") -1)
    _
    (else
      (Utilities|Array|RemoveItem _inventory "BlindnessPotion")))
  (Utilities|Casting|CastToPlayerPawn (Components|GetOwner))
  (Variables|Default|SetCurrentHoldingPotion "None")
  (if (== _playerindex 0)
    (bind _asliam_game_mode (Utilities|Casting|CastToLiam_GameMode _returnvalue))
    (Default|UpdateCurrentPotion (Variables|/Game/Liam/Liam_GameMode.Liam_GameMode_C|GetInventory_PL1 _asliam_game_mode))
    (elif (== _playerindex 1)
      (bind _asliam_game_mode_2 (Utilities|Casting|CastToLiam_GameMode _returnvalue))
      (Default|UpdateCurrentPotion (Variables|/Game/Liam/Liam_GameMode.Liam_GameMode_C|GetInventory_PL2 _asliam_game_mode_2)))))