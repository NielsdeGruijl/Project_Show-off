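; BP_Player is the player character Blueprint, providing basic move, look and jump controls through Enhanced Input.
; On BeginPlay it adds the IMC_GameInput mapping context to its player controller's local input subsystem.
; Look input feeds controller yaw and pitch, while move input follows control rotation with pitch zeroed, so looking up or down does not tilt movement.
; Jump starts on the action's Triggered event and stops on Completed.
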(event Input|EnhancedActionEvents|EnhancedInputActionIA_JumpCharacter
  (params (ActionValue :type Boolean) (ElapsedSeconds :type Float%20%28double-precision%29) (TriggeredSeconds :type Float%20%28double-precision%29) (InputAction :type Input%20Action%20Object%20Reference :default "/Game/Liam/Character/Input/IA_JumpCharacter.IA_JumpCharacter"))
  (:Triggered
    (Character|Jump))
  (:Completed
    (Character|StopJumping)))

(event Input|EnhancedActionEvents|EnhancedInputActionIA_LookCharacter
  (params (ActionValue :type Vector%202D%20Structure) (ElapsedSeconds :type Float%20%28double-precision%29) (TriggeredSeconds :type Float%20%28double-precision%29) (InputAction :type Input%20Action%20Object%20Reference :default "/Game/Liam/Character/Input/IA_LookCharacter.IA_LookCharacter"))
  (:Triggered
    (Pawn|Input|AddControllerYawInput (.x ActionValue))
    (Pawn|Input|AddControllerPitchInput (.y ActionValue))))

(event Input|EnhancedActionEvents|EnhancedInputActionIA_MoveCharacter
  (params (ActionValue :type Vector :default "0, 0, 0") (ElapsedSeconds :type Float%20%28double-precision%29) (TriggeredSeconds :type Float%20%28double-precision%29) (InputAction :type Input%20Action%20Object%20Reference :default "/Game/Liam/Character/Input/IA_MoveCharacter.IA_MoveCharacter"))
  (bind _returnvalue (Pawn|GetController))
  (bind _returnvalue_2 (Pawn|GetControlRotation _returnvalue :!class /Script/Engine.Controller))
  (:Triggered
    (Pawn|Input|AddMovementInput (Math|Vector|GetRightVector (Math|Rotator|MakeRotator (.roll _returnvalue_2) 0.0 (.yaw _returnvalue_2))) (.x ActionValue) false)
    (Pawn|Input|AddMovementInput (Math|Vector|GetForwardVector (Math|Rotator|MakeRotator 0.0 0.0 (.yaw (Pawn|GetControlRotation (Pawn|GetController) :!class /Script/Engine.Controller)))) (.y ActionValue) false)))

(event EventBeginPlay
  (bind _asplayer_controller (Utilities|Casting|CastToPlayerController (Pawn|GetController)))
  (Utilities|IsValid (PlayerController|LocalPlayerSubsystems|GetEnhancedInputLocalPlayerSubsystem _asplayer_controller)
    (:Is%20Valid
      (Input|AddMappingContext (PlayerController|LocalPlayerSubsystems|GetEnhancedInputLocalPlayerSubsystem _asplayer_controller) "/Game/Liam/Character/Input/IMC_GameInput.IMC_GameInput" 0 "(bIgnoreAllPressedKeysUntilRelease=True,bForceImmediately=False)"))))

(fn ConstructionScript)